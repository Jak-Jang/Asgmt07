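; BP_Test2 is a player-controlled drone pawn that registers the IMC_Drone Enhanced Input context when possessed.
; Move, look, lift and tilt inputs apply transform offsets and rotations directly, with look yawing the actor and pitching the spring arm.
; Horizontal movement drops to a tenth when the capsule reports vertical velocity.
; Releasing lift starts a hand-rolled fall on Tick, whose speed compounds each frame until lift resumes.
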(event Input|EnhancedActionEvents|EnhancedInputActionIA_DroneMove
  (params (ActionValue :type Vector%202D%20Structure) (ElapsedSeconds :type Float%20%28double-precision%29) (TriggeredSeconds :type Float%20%28double-precision%29) (InputAction :type Input%20Action%20Object%20Reference :default "/Game/Inputs/IA_DroneMove.IA_DroneMove"))
  (bind _movespeed (Variables|Default|GetMoveSpeed))
  (if (== (.z (Transformation|GetComponentVelocity (Variables|Default|GetCapsule))) 0.0)
    (Transformation|AddActorLocalOffset (Math|Vector|MakeVector (* (* (.x ActionValue) _movespeed) (stale EventTick DeltaSeconds)) (* (* (.y ActionValue) _movespeed) (stale EventTick DeltaSeconds)) 0.0) true false)
    (else
      (Transformation|AddActorLocalOffset (Math|Vector|MakeVector (* (* (* (.x ActionValue) _movespeed) (stale EventTick DeltaSeconds)) 0.1) (* (* (* (.y ActionValue) _movespeed) (stale EventTick DeltaSeconds)) 0.1) 0.0) true false))))

(event Input|EnhancedActionEvents|EnhancedInputActionIA_DroneLook
  (params (ActionValue :type Vector%202D%20Structure) (ElapsedSeconds :type Float%20%28double-precision%29) (TriggeredSeconds :type Float%20%28double-precision%29) (InputAction :type Input%20Action%20Object%20Reference :default "/Game/Inputs/IA_DroneLook.IA_DroneLook"))
  (bind _lookspeed (Variables|Default|GetLookSpeed))
  (Class|Actor|AddActorWorldRotation (Math|Rotator|MakeRotator 0.0 0.0 (* (* (.x ActionValue) _lookspeed) (stale EventTick DeltaSeconds))))
  (Transformation|AddLocalRotation (Variables|Default|GetSpringArm) (Math|Rotator|MakeRotator 0.0 (* (* (.y ActionValue) _lookspeed) (stale EventTick DeltaSeconds)) 0.0) false false))

(event Input|EnhancedActionEvents|EnhancedInputActionIA_DroneLift
  (params (ActionValue :type Boolean) (ElapsedSeconds :type Float%20%28double-precision%29) (TriggeredSeconds :type Float%20%28double-precision%29) (InputAction :type Input%20Action%20Object%20Reference :default "/Game/Inputs/IA_DroneLift.IA_DroneLift"))
  (:Triggered
    (Variables|Default|SetIsFalling false)
    (if ActionValue
      (Transformation|AddActorLocalOffset (Math|Vector|MakeVector 0.0 0.0 (* (Variables|Default|GetLiftSpeed) (stale EventTick DeltaSeconds))) true false)))
  (:Completed
    (Variables|Default|SetIsFalling true)
    (Variables|Default|SetFalling -9.8e+02)))

(event Input|EnhancedActionEvents|EnhancedInputActionIA_DroneTilting
  (params (ActionValue :type Float%20%28double-precision%29) (ElapsedSeconds :type Float%20%28double-precision%29) (TriggeredSeconds :type Float%20%28double-precision%29) (InputAction :type Input%20Action%20Object%20Reference :default "/Game/Inputs/IA_DroneTilting.IA_DroneTilting"))
  (Transformation|AddActorLocalRotation (Math|Rotator|MakeRotator 0.0 (* (* ActionValue (Variables|Default|GetRotateSpeed)) (stale EventTick DeltaSeconds)) 0.0) false false))

(event EventTick
  (params (DeltaSeconds :type Float%20%28single-precision%29))
  (if (Variables|Default|GetIsFalling)
    (Transformation|AddActorWorldOffset (Math|Vector|MakeVector 0.0 0.0 (* (Variables|Default|GetFalling) DeltaSeconds)) true)
    (Variables|Default|SetFalling (+ (* DeltaSeconds (Variables|Default|GetFalling)) (Variables|Default|GetFalling)))))

(event EventControllerChanged
  (params (OldController :type Controller%20Object%20Reference) (NewController :type Controller%20Object%20Reference))
  (bind _asplayer_controller (Utilities|Casting|CastToPlayerController NewController))
  (Input|AddMappingContext (PlayerController|LocalPlayerSubsystems|GetEnhancedInputLocalPlayerSubsystem _asplayer_controller) "/Game/Inputs/IMC_Drone.IMC_Drone" 0 "(bIgnoreAllPressedKeysUntilRelease=True,bForceImmediately=False,bNotifyUserSettings=False)"))

(fn ConstructionScript)