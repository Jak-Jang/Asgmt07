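; BP_Test is a test pawn that a player moves with Enhanced Input.
; When its controller changes to a PlayerController, it adds the IMC_Move mapping context to that player's input subsystem.
; IA_Move offsets the actor along local X and Y by the input value scaled by MoveSpeed and delta seconds.
; Tick and the construction script are empty, and a leftover input-component setup never runs.
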(event Input|EnhancedActionEvents|EnhancedInputActionIA_Move
  (params (ActionValue :type Vector%202D%20Structure) (ElapsedSeconds :type Float%20%28double-precision%29) (TriggeredSeconds :type Float%20%28double-precision%29) (InputAction :type Input%20Action%20Object%20Reference :default "/Game/Inputs/IA_Move.IA_Move"))
  (bind _movespeed (Variables|Default|GetMoveSpeed))
  (Transformation|AddActorLocalOffset (Math|Vector|MakeVector (* (* (.x ActionValue) _movespeed) (stale EventTick DeltaSeconds)) (* (* (.y ActionValue) _movespeed) (stale EventTick DeltaSeconds)) 0.0) false false))

(event EventTick
  (params (DeltaSeconds :type Float%20%28single-precision%29)))

(event EventControllerChanged
  (params (OldController :type Controller%20Object%20Reference) (NewController :type Controller%20Object%20Reference))
  (bind _asplayer_controller (Utilities|Casting|CastToPlayerController NewController))
  (Input|AddMappingContext (PlayerController|LocalPlayerSubsystems|GetEnhancedInputLocalPlayerSubsystem _asplayer_controller) "/Game/Inputs/IMC_Move.IMC_Move" 0 "(bIgnoreAllPressedKeysUntilRelease=True,bForceImmediately=False,bNotifyUserSettings=False)"))

(fn ConstructionScript)